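; Joust enemy buzzard character whose rider tier (Bounder, Hunter or Shadow Lord) follows EggID, which scales its speed and climb rate.
; Tick drives it sideways while small launches steer its height just above the player or, when riderless, toward its egg.
; Hits flip its direction, and UnmountJouster drops a next-tier egg and marks it defeated.
; WrapEffect wraps it across screen edges or destroys it once defeated, while MountJouster seats a rider.
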(event OnComponentHit(CapsuleComponent)
  (params (HitComponent :type Primitive%20Component%20Object%20Reference) (OtherActor :type Actor%20Object%20Reference) (OtherComp :type Primitive%20Component%20Object%20Reference) (NormalImpulse :type Vector :default "0, 0, 0") (Hit :type Hit%20Result%20Structure%20%28by%20ref%29))
  (if (Variables|Default|GetbhasMount)
    (Utilities|FlowControl|DoOnce false :!label _label
      (:Completed
        (Utilities|FlowControl|FlipFlop
          (:A
            (Variables|Default|SetScale%20Value -1.0))
          (:B
            (Variables|Default|SetScale%20Value 1.0)))
        (Audio|PlaySound2D "/Game/Assets/SFX/Joust_Thunk_Sound.Joust_Thunk_Sound" 1.0 1.0 0.0 0 0)
        (Utilities|FlowControl|Delay 2.2)
        (goto _label Reset)))))

(event EventMountJouster
  (params (EggID :type Integer))
  (bind _capsulecomponent (Variables|Default|GetCapsuleComponent))
  (Variables|Default|SetEgg%20ID EggID)
  (Development|SetHiddeninGame (Variables|Default|GetPaperSprite) false false)
  (Variables|Default|SetbhasMount true)
  (Sprite|SetFlipbook (Variables|Default|GetSprite) "/Game/Assets/Textures/Buzzard/Fly/T_Buzzard_Fly.T_Buzzard_Fly")
  (Transformation|SetRelativeLocation (Variables|Default|GetPaperSprite) "7.000000,0.000000,7.000000" false false)
  (Variables|/Script/Engine.CharacterMovementComponent|SetGravityScale (Variables|Character|GetCharacterMovement) 0.0)
  (Rendering|Components|Sprite|SetSprite (Variables|Default|GetPaperSprite) (Utilities|Select :Index (Variables|Default|GetEgg%20ID) :Option%200 "/Game/Assets/Textures/Bounder/TX_Bounder_Idle_01_Sprite.TX_Bounder_Idle_01_Sprite" :Option%201 "/Game/Assets/Textures/Hunter/TX_Hunter_Idle_01_Sprite.TX_Hunter_Idle_01_Sprite" :Option%202 "/Game/Assets/Textures/ShadowLord/TX_ShadowLord_Idle_01_Sprite.TX_ShadowLord_Idle_01_Sprite"))
  (Collision|SetCollisionResponsetoChannel _capsulecomponent "ECC_GameTraceChannel1" "ECR_Block")
  (Collision|SetCollisionResponsetoChannel _capsulecomponent "ECC_GameTraceChannel2" "ECR_Block")
  (Collision|SetCollisionResponsetoChannel _capsulecomponent "ECC_GameTraceChannel3" "ECR_Ignore"))

(event EventTick
  (params (DeltaSeconds :type Float%20%28single-precision%29))
  (bind _returnvalue (Game|Player|GetPlayerPawn 0))
  (bind _returnvalue_2 (Transformation|GetActorLocation))
  (bind _returnvalue_3 (Transformation|GetActorLocation))
  (bind _bp_egg (Variables|Default|GetBP_Egg))
  (bind _egg_id (Variables|Default|GetEgg%20ID))
  (bind _scale_value (Variables|Default|GetScale%20Value))
  (bind _returnvalue_4 (Transformation|GetActorLocation _returnvalue))
  (bind _returnvalue_5 (Transformation|GetActorLocation _bp_egg))
  (bind _returnvalue_6 (Utilities|Select :Index _egg_id :Option%200 "0.000000,0.000000,-0.500000" :Option%201 "0.000000,0.000000,-1.000000" :Option%202 "0.000000,0.000000,-1.500000"))
  (bind _returnvalue_7 (+ (.z _returnvalue_4) 8.0))
  (Pawn|Input|AddMovementInput (Transformation|GetActorForwardVector) _scale_value false)
  (Transformation|SetRelativeRotation (Variables|Default|GetSprite) (Math|Rotator|SelectRotator "0.000000,180.000000,0.000000" "0, 0, 0" (== _scale_value -1.0)) false false)
  (Utilities|FlowControl|Sequence
    (:then_0
      (if (Variables|Default|GetbhasMount)
        (if (Math|Float|NearlyEqual(Float) (.z _returnvalue_2) _returnvalue_7 (Utilities|Select :Index (Variables|Default|GetEgg%20ID) :Option%200 0.25 :Option%201 0.1 :Option%202 0.0))
          (Character|LaunchCharacter _returnvalue_6 false false)
          (elif (> (.z _returnvalue_2) _returnvalue_7)
            (Character|LaunchCharacter _returnvalue_6 false false)
            (else
              (Character|LaunchCharacter (Utilities|Select :Index (Variables|Default|GetEgg%20ID) :Option%200 "0.000000,0.000000,0.500000" :Option%201 "0.000000,0.000000,1.000000" :Option%202 "0.000000,0.000000,1.500000") false false))))
        (else
          (Variables|Default|GetBP_Egg
            (:then
              (Sprite|SetFlipbook (Variables|Default|GetSprite) "/Game/Assets/Textures/Buzzard/Fly/T_Buzzard_Fly.T_Buzzard_Fly")
              (Variables|/Script/Engine.CharacterMovementComponent|SetGravityScale (Variables|Character|GetCharacterMovement) 0.0)
              (if (Math|Float|NearlyEqual(Float) (.z _returnvalue_3) (.z _returnvalue_5) 0.0)
                (Character|LaunchCharacter (Utilities|Select :Index (Variables|Default|GetEgg%20ID) :Option%200 "0.000000,0.000000,-0.500000" :Option%201 "0.000000,0.000000,-1.000000" :Option%202 "0.000000,0.000000,-1.500000") false false :!label _label)
                (elif (> (.z _returnvalue_3) (.z _returnvalue_5))
                  (goto _label)
                  (else
                    (Character|LaunchCharacter (Utilities|Select :Index (Variables|Default|GetEgg%20ID) :Option%200 "0.000000,0.000000,0.500000" :Option%201 "0.000000,0.000000,1.000000" :Option%202 "0.000000,0.000000,1.500000") false false)))))
            (:else
              (Variables|Default|SetbisDefeated true))))))
    (:then_1
      (Utilities|WrapEffect))))

(event EventBeginPlay
  (bind _charactermovement (Variables|Character|GetCharacterMovement))
  (Transformation|SetRelativeLocation (Variables|Default|GetPaperSprite) "7.000000,0.000000,14.000000" false false)
  (Variables|/Script/Engine.CharacterMovementComponent|SetMaxWalkSpeed _charactermovement (Utilities|Select :Index (Variables|Default|GetEgg%20ID) :Option%200 75.0 :Option%201 275.0 :Option%202 4.5e+02))
  (Variables|/Script/Engine.CharacterMovementComponent|SetAirControl _charactermovement (Utilities|Select :Index (Variables|Default|GetEgg%20ID) :Option%200 0.1 :Option%201 1.0 :Option%202 8.0)))

(event EventUnmountJouster
  (bind _capsulecomponent (Variables|Default|GetCapsuleComponent))
  (Utilities|FlowControl|DoOnce false
    (:Completed
      (Audio|PlaySound2D "/Game/Assets/SFX/Joust_Death_Sound.Joust_Death_Sound" 1.0 1.0 0.0 0 0)
      (Development|SetHiddeninGame (Variables|Default|GetPaperSprite) true false)
      (Variables|Default|SetbhasMount false)
      (Character|LaunchCharacter (* (Transformation|GetActorForwardVector) 1e+02) true true)
      (Variables|/Script/Engine.CharacterMovementComponent|SetMaxWalkSpeed (Variables|Character|GetCharacterMovement) 1e+02)
      (Game|SpawnActorfromClass "/Game/Game/Core/Actors/Egg/BP_Egg.BP_Egg_C" (Math|Transform|MakeTransform (Transformation|GetActorLocation) "0.000000,90.000000,0.000000" "1.000000,1.000000,1.000000") "AlwaysSpawn" "MultiplyWithRoot" 0 (+ (Variables|Default|GetEgg%20ID) 1) 0)
      (Collision|SetCollisionResponsetoChannel _capsulecomponent "ECC_GameTraceChannel1" "ECR_Ignore")
      (Collision|SetCollisionResponsetoChannel _capsulecomponent "ECC_GameTraceChannel3" "ECR_Ignore")
      (Collision|SetCollisionResponsetoChannel _capsulecomponent "ECC_GameTraceChannel2" "ECR_Ignore")
      (Variables|Default|SetbisDefeated true))))

(fn ConstructionScript
  (|CallParentFunction))