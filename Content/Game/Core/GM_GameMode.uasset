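; Game mode for a Joust-style game that tracks score, multiplier and lives, and handles game over.
; On BeginPlay it forces a windowed resolution and frame rate cap, then binds to its removed-health event.
; RemoveHealth fires that event; negative lives hide platforms, destroy players, buzzards, eggs and spawn platforms, show the game-over widget and endlessly loop random sounds.
; AddPoints adds raw points and can raise the clamped multiplier without applying it.
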(event Custom|Event_RemovedHealth_Event
  (params (currentHealth :type Integer))
  (if (< currentHealth 0)
    (bind _outactors (Actor|GetAllActorswithTag "Platform"))
    (for _array_element _outactors
      (Rendering|SetActorHiddenInGame _array_element true))
    (bind _outactors_2 (Actor|GetAllActorsOfClass "/Game/Game/AI/Jousts/BP_Buzzard.BP_Buzzard_C"))
    (for _array_element_2 _outactors_2
      (Actor|DestroyActor _array_element_2))
    (bind _outactors_3 (Actor|GetAllActorsOfClass "/Game/Game/Core/Actors/Egg/BP_Egg.BP_Egg_C"))
    (for _array_element_3 _outactors_3
      (Actor|DestroyActor _array_element_3))
    (bind _outactors_4 (Actor|GetAllActorsOfClass "/Game/Game/Core/Actors/SpawnPlatform/BP_SpawnPlatform.BP_SpawnPlatform_C"))
    (for _array_element_4 _outactors_4
      (Actor|DestroyActor _array_element_4))
    (bind _outactors_5 (Actor|GetAllActorsOfClass "/Game/Game/Player/BP_MyPlayer.BP_MyPlayer_C"))
    (for _array_element_5 _outactors_5
      (Actor|DestroyActor _array_element_5))
    (bind _returnvalue (UserInterface|CreateWidget "/Game/Menu/GameMenu/WBP_GameOver.WBP_GameOver_C"))
    (UserInterface|Viewport|AddtoViewport _returnvalue 0)
    (Audio|PlaySound2D (Utilities|Select :Index (Math|Random|RandomIntegerinRange 0 1) :Option%200 "/Game/Assets/SFX/Joust_GameOver.Joust_GameOver" :Option%201 "/Game/Assets/SFX/Joust_Lava_Sound.Joust_Lava_Sound") 1.0 1.0 0.0 0 0 :!label _label)
    (Utilities|FlowControl|Delay (Math|Random|RandomFloatinRange 0.5 3.0))
    (goto _label)))

(event EventBeginPlay
  (bind _returnvalue (Settings|GetGameUserSettings))
  (Class|GameUserSettings|SetFrameRateLimit _returnvalue 6e+01)
  (Class|GameUserSettings|SetScreenResolution _returnvalue (Utilities|Struct|MakeIntPoint 1280 960))
  (Class|GameUserSettings|SetFullscreenMode _returnvalue "Windowed")
  (Class|GameUserSettings|ApplyResolutionSettings _returnvalue false)
  (Class|GameUserSettings|ApplySettings _returnvalue true)
  (EventDispatchers|BindEventtoEventRemovedHealth (delegate Custom|Event_RemovedHealth_Event)))

(fn ConstructionScript)

(fn AddPoints
  (params (addedPoints :type Integer) (shouldMultiplier :type Boolean))
  (Variables|Default|SetPlayerScore (+ (Variables|Default|GetPlayerScore) addedPoints))
  (if shouldMultiplier
    (Variables|Default|SetScoreMultiplier (Math|Integer|Clamp(Integer) (+ (Variables|Default|GetScoreMultiplier) 1) 1 4))))

(fn RemoveHealth
  (params (removedHealth :type Integer))
  (bind _output_get (Variables|Default|SetPlayerLives (- (Variables|Default|GetPlayerLives) removedHealth)))
  (Default|CallEventRemovedHealth _output_get))