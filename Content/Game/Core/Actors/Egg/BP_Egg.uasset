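; Joust-style egg pickup that hatches into a Bounder, Hunter or Shadow Lord according to EggID.
; Timed BeginPlay sequence plays the hatch flipbook, shows the idle rider, then spawns a BP_Bounder at a fixed X/Y at egg height, passing itself as BPEgg.
; Player overlap awards EggID-based points, fewer once hatched, and destroys it.
; A riderless BP_JoustMaster overlapping a hatched egg calls MountJouster with EggID and consumes it.
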(event OnComponentBeginOverlap(PickUp)
  (params (OverlappedComponent :type Primitive%20Component%20Object%20Reference) (OtherActor :type Actor%20Object%20Reference) (OtherComp :type Primitive%20Component%20Object%20Reference) (OtherBodyIndex :type Integer) (bFromSweep :type Boolean) (SweepResult :type Hit%20Result%20Structure%20%28by%20ref%29))
  (Utilities|Casting|CastToBP_MyPlayer OtherActor
    (:then
      (Audio|PlaySound2D "/Game/Assets/SFX/Joust_Egg_Sound.Joust_Egg_Sound" 1.0 1.0 0.0 0 0)
      (Default|AddPoints (Variables|Default|GetAs%20GM%20Game%20Mode) (Math|Integer|SelectInt (Utilities|Select :Index (Variables|Default|GetEggID) :Option%200 250 :Option%201 500 :Option%202 750) (Utilities|Select :Index (Variables|Default|GetEggID) :Option%200 500 :Option%201 750 :Option%202 1000) (Variables|Default|GetbisHatched)))
      (Actor|DestroyActor))
    (:CastFailed
      (bind _asbp_joust_master (Utilities|Casting|CastToBP_JoustMaster OtherActor))
      (if (Variables|Default|GetbisHatched)
        (if (not (Variables|/Game/Game/AI/Jousts/BP_JoustMaster.BP_JoustMaster_C|GetbhasMount _asbp_joust_master))
          (Default|MountJouster _asbp_joust_master (Variables|Default|GetEggID))
          (Actor|DestroyActor))))))

(event EventBeginPlay
  (bind _paperflipbook (Variables|Default|GetPaperFlipbook))
  (bind _asgm_game_mode (Utilities|Casting|CastToGM_GameMode (Game|GetGameMode)))
  (Variables|Default|SetAs%20GM%20Game%20Mode _asgm_game_mode)
  (Utilities|FlowControl|Delay 5.0)
  (Components|Sphere|SetSphereRadius (Variables|Default|GetPickUp) 13.0 true)
  (Sprite|SetFlipbook _paperflipbook "/Game/Assets/Textures/Egg/Hatch/TX_Egg_Hatch.TX_Egg_Hatch")
  (Components|Timeline|SetLooping _paperflipbook false)
  (Utilities|FlowControl|Delay 0.3)
  (Sprite|SetFlipbook (Variables|Default|GetPaperFlipbook) (Utilities|Select :Index (Variables|Default|GetEggID) :Option%200 "/Game/Assets/Textures/Bounder/TX_Bounder_Idle.TX_Bounder_Idle" :Option%201 "/Game/Assets/Textures/Hunter/TX_Hunter_Idle.TX_Hunter_Idle" :Option%202 "/Game/Assets/Textures/ShadowLord/TX_ShadowLord_Idle.TX_ShadowLord_Idle"))
  (Variables|Default|SetbisHatched true)
  (Collision|SetCollisionResponsetoChannel (Variables|Default|GetRoot) "ECC_GameTraceChannel2" "ECR_Overlap")
  (Utilities|FlowControl|Delay 4.0)
  (Game|SpawnActorfromClass "/Game/Game/AI/Jousts/BP_Bounder.BP_Bounder_C" (Math|Transform|MakeTransform (Math|Vector|MakeVector 171.813278 -189.95993 (.z (Transformation|GetActorLocation))) "0.000000,90.000000,0.000000" "1.000000,1.000000,1.000000") "AlwaysSpawn" "MultiplyWithRoot" 0 self 0))

(fn ConstructionScript)