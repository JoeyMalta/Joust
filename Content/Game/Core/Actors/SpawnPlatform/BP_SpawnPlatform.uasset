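; BP_SpawnPlatform is a Joust-style spawn point that creates the player or buzzard enemies at its flipbook's location.
; On Tick, paired DoOnce gates clear its tags when the player comes within range and add "Available" once the player moves away.
; SpawnBuzzard mounts a jouster by egg ID and plays a sound.
; SpawnPlayer applies spawn protection and removes one health through GM_GameMode.
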(event Custom|SpawnBuzzard
  (params (EggID :type Integer))
  (bind _returnvalue (Game|SpawnActorfromClass "/Game/Game/AI/Jousts/BP_Buzzard.BP_Buzzard_C" (Math|Transform|MakeTransform (Transformation|GetWorldLocation (Variables|Default|GetPaperFlipbook)) "0.000000,90.000000,0.000000" "1.000000,1.000000,1.000000") "AlwaysSpawn" "MultiplyWithRoot" 0 0 0))
  (Default|MountJouster _returnvalue EggID)
  (Audio|PlaySound2D "/Game/Assets/SFX/Joust_EnemySpawn.Joust_EnemySpawn" 0.5 1.0 0.0 0 0))

(event Custom|SpawnPlayer
  (bind _returnvalue (Game|SpawnActorfromClass "/Game/Game/Player/BP_MyPlayer.BP_MyPlayer_C" (Math|Transform|MakeTransform (Transformation|GetWorldLocation (Variables|Default|GetPaperFlipbook)) "0.000000,90.000000,0.000000" "1.000000,1.000000,1.000000") "AlwaysSpawn" "MultiplyWithRoot" 0 true 0))
  (Default|ApplySpawnProtection _returnvalue)
  (bind _asgm_game_mode (Utilities|Casting|CastToGM_GameMode (Game|GetGameMode)))
  (Default|RemoveHealth _asgm_game_mode 1))

(event EventTick
  (params (DeltaSeconds :type Float%20%28single-precision%29))
  (bind _asbp_my_player (Utilities|Casting|CastToBP_MyPlayer (Game|Player|GetPlayerPawn 0)))
  (if (< (Transformation|GetDistanceTo _asbp_my_player) 1e+02)
    (Utilities|FlowControl|DoOnce false :!label _label
      (:Completed
        (Utilities|Array|Clear (Variables|Actor|GetTags))
        (goto _label_2 Reset)))
    (else
      (Utilities|FlowControl|DoOnce false :!label _label_2
        (:Completed
          (Utilities|Array|Add (Variables|Actor|GetTags) "Available")
          (goto _label Reset))))))

(event EventBeginPlay)

(fn ConstructionScript)