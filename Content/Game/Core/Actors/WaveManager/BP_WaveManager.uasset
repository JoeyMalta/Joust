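; Wave manager that spawns each numbered wave of buzzard enemies and handles player respawns.
; StartWave increments the wave and reads its Bounder, Hunter and Shadow Lord counts from DT_WaveStruct.
; A delayed-loop macro spawns each type in sequence, picking a random "Available" spawn platform each time.
; RespawnPlayer waits briefly, then, unless health is below zero, resets the score multiplier and spawns at the first cached platform.
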(event Custom|StartWave
  (bind _result (Math|Integer|IncrementInt (Variables|Default|GetCurrentWave))
    (:%20%20
      (Variables|Default|SetCurrentWave _result)
      (bind _returnvalue (Utilities|GetDataTableRow "/Game/Game/Core/Actors/WaveManager/DT_WaveStruct.DT_WaveStruct" (Utilities|String|StringToName (Utilities|String|ToString(Integer) (Variables|Default|GetCurrentWave))))
        (:then
          (Utilities|ForLoopwithDelay 0 (- (.BounderAmount (Utilities|Struct|BreakF_WaveStruct _returnvalue)) 1) 1.5
            (:LoopBody
              (bind _outactors (Actor|GetAllActorsOfClasswithTag "/Game/Game/Core/Actors/SpawnPlatform/BP_SpawnPlatform.BP_SpawnPlatform_C" "Available"))
              (bind _output_get (Variables|Default|SetSpawnPlatforms _outactors))
              (Utilities|Array|Shuffle _output_get)
              (Default|SpawnBuzzard (Utilities|Array|Get(acopy) _output_get)))
            (:Completed
              (if (== (.HunterAmount (Utilities|Struct|BreakF_WaveStruct _returnvalue)) 0)
                (if (not (== (.ShadowLordAmount (Utilities|Struct|BreakF_WaveStruct _returnvalue)) 0)) :!label _label
                  (Utilities|ForLoopwithDelay 0 (- (.ShadowLordAmount (Utilities|Struct|BreakF_WaveStruct _returnvalue)) 1) 1.5
                    (:LoopBody
                      (bind _outactors_2 (Actor|GetAllActorsOfClasswithTag "/Game/Game/Core/Actors/SpawnPlatform/BP_SpawnPlatform.BP_SpawnPlatform_C" "Available"))
                      (bind _output_get_2 (Variables|Default|SetSpawnPlatforms _outactors_2))
                      (Utilities|Array|Shuffle _output_get_2)
                      (Default|SpawnBuzzard (Utilities|Array|Get(acopy) _output_get_2) 2))))
                (else
                  (Utilities|ForLoopwithDelay 0 (- (.HunterAmount (Utilities|Struct|BreakF_WaveStruct _returnvalue)) 1) 1.5
                    (:LoopBody
                      (bind _outactors_3 (Actor|GetAllActorsOfClasswithTag "/Game/Game/Core/Actors/SpawnPlatform/BP_SpawnPlatform.BP_SpawnPlatform_C" "Available"))
                      (bind _output_get_3 (Variables|Default|SetSpawnPlatforms _outactors_3))
                      (Utilities|Array|Shuffle _output_get_3)
                      (Default|SpawnBuzzard (Utilities|Array|Get(acopy) _output_get_3) 1))
                    (:Completed
                      (goto _label))))))))))))

(event Custom|RespawnPlayer
  (Utilities|FlowControl|Delay 0.5)
  (bind _asgm_game_mode (Utilities|Casting|CastToGM_GameMode (Game|GetGameMode)))
  (if (not (< (Variables|/Game/Game/Core/GM_GameMode.GM_GameMode_C|GetPlayerHealth _asgm_game_mode) 0))
    (Variables|/Game/Game/Core/GM_GameMode.GM_GameMode_C|SetScoreMultiplier _asgm_game_mode 1)
    (Default|SpawnPlayer (Utilities|Array|Get(acopy) (Variables|Default|GetSpawnPlatforms)))))

(fn ConstructionScript)