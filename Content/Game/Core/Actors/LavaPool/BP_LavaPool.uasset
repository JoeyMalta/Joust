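; Lava pool actor that plays a Joust-style intro sequence when InitSequence is called.
; The Init timeline lowers a black plane as a start sound plays, then unhides all Platform-tagged actors and starts LavaSequence.
; LavaSequence uses a second timeline to slide the lava sprite to its relative origin.
; A Delay and DoN on that timeline's update space out and cap the repeated lava sound.
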(event Custom|InitSequence
  (bind _blackplane (Variables|Default|GetBlackPlane)
    (:then
      (Variables|Default|SetRelative%20Location (Variables|/Script/Engine.SceneComponent|GetRelativeLocation _blackplane))
      (Components|Timeline|SetPlayRate (Variables|Default|GetInit) (/ 1.0 1.5))
      (Audio|PlaySound2D "/Game/Assets/SFX/Joust_Start_Sound.Joust_Start_Sound" 1.0 1.0 0.0 0 0)
      (bind _alpha (Timeline|Init PlayFromStart)
        (:Update
          (Transformation|SetRelativeLocation (Variables|Default|GetBlackPlane) (Math|Vector|Lerp(Vector) (Variables|Default|GetRelative%20Location) (Math|Vector|MakeVector (.x (Variables|Default|GetRelative%20Location)) (.y (Variables|Default|GetRelative%20Location)) (- (.z (Variables|Default|GetRelative%20Location)) 7e+01)) _alpha) false false))
        (:Finished
          (CallFunction|LavaSequence)
          (bind _outactors (Actor|GetAllActorswithTag "Platform"))
          (for _array_element _outactors
            (Rendering|SetActorHiddenInGame _array_element false)))))
    (:else)))

(event Custom|LavaSequence
  (Variables|Default|SetRelative%20Location_0 (Variables|/Script/Engine.SceneComponent|GetRelativeLocation (Variables|Default|GetPaperSprite)))
  (Components|Timeline|SetPlayRate (Variables|Default|GetLava) (/ 1.0 3.5))
  (bind _alpha (Timeline|Lava PlayFromStart)
    (:Update
      (Transformation|SetRelativeLocation (Variables|Default|GetPaperSprite) (Math|Vector|Lerp(Vector) (Variables|Default|GetRelative%20Location_0) "0, 0, 0" _alpha) false false)
      (Utilities|FlowControl|Delay 0.9)
      (Utilities|FlowControl|DoN 3
        (:Exit
          (Audio|PlaySound2D "/Game/Assets/SFX/Joust_Lava_Sound.Joust_Lava_Sound" 1.0 1.0 0.0 0 0))))))

(fn ConstructionScript)