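; Menu pawn that handles arcade-style coin and start input for the main menu.
; Key 5 adds a credit to GI_GameInstance; key 1 requires at least one credit, otherwise printing a prompt.
; Starting possesses BP_MyPlayer, removes all widgets and runs BP_LavaPool's InitSequence.
; Numpad keys switch WB_MainMenu pages, with NumPadThree bound three times to conflicting indices.
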(event Input|KeyboardEvents|NumPadThree
  (params (Key :type Key%20Structure :default "None"))
  (:Pressed
    (bind _foundwidgets (Widget|GetAllWidgetsOfClass "/Game/Menu/MainMenu/WB_MainMenu.WB_MainMenu_C" false))
    (Default|SwitchWidget (Utilities|Array|Get(acopy) _foundwidgets) 3)))

(event Input|KeyboardEvents|5
  (params (Key :type Key%20Structure :default "None"))
  (:Pressed
    (bind _asgi_game_instance (Utilities|Casting|CastToGI_GameInstance (Game|GetGameInstance)))
    (Default|AddCredit _asgi_game_instance)))

(event Input|KeyboardEvents|1
  (params (Key :type Key%20Structure :default "None"))
  (:Pressed
    (bind _asgi_game_instance (Utilities|Casting|CastToGI_GameInstance (Game|GetGameInstance)))
    (if (>= (Variables|/Game/Game/Core/GI_GameInstance.GI_GameInstance_C|GetCredits _asgi_game_instance) 1)
      (bind _returnvalue (Actor|GetActorOfClass "/Game/Game/Player/BP_MyPlayer.BP_MyPlayer_C"))
      (Pawn|Possess (Game|GetPlayerController 0) _returnvalue)
      (Viewport|RemoveAllWidgets)
      (bind _returnvalue_2 (Actor|GetActorOfClass "/Game/Game/Core/Actors/LavaPool/BP_LavaPool.BP_LavaPool_C"))
      (Default|InitSequence _returnvalue_2)
      (else
        (Development|PrintString "PRESS \"5\" TO ADD CREDITS" true true "(R=1.000000,G=0.837292,B=0.000000,A=1.000000)")))))

(event Input|KeyboardEvents|2
  (params (Key :type Key%20Structure :default "None")))

(event Input|KeyboardEvents|NumPadOne
  (params (Key :type Key%20Structure :default "None"))
  (:Pressed
    (bind _foundwidgets (Widget|GetAllWidgetsOfClass "/Game/Menu/MainMenu/WB_MainMenu.WB_MainMenu_C" false))
    (Default|SwitchWidget (Utilities|Array|Get(acopy) _foundwidgets))))

(event Input|KeyboardEvents|NumPadTwo
  (params (Key :type Key%20Structure :default "None"))
  (:Pressed
    (bind _foundwidgets (Widget|GetAllWidgetsOfClass "/Game/Menu/MainMenu/WB_MainMenu.WB_MainMenu_C" false))
    (Default|SwitchWidget (Utilities|Array|Get(acopy) _foundwidgets) 1)))

(event Input|KeyboardEvents|NumPadThree
  (params (Key :type Key%20Structure :default "None"))
  (:Pressed
    (bind _foundwidgets (Widget|GetAllWidgetsOfClass "/Game/Menu/MainMenu/WB_MainMenu.WB_MainMenu_C" false))
    (Default|SwitchWidget (Utilities|Array|Get(acopy) _foundwidgets) 2)))

(event Input|KeyboardEvents|NumPadThree
  (params (Key :type Key%20Structure :default "None"))
  (:Pressed
    (bind _foundwidgets (Widget|GetAllWidgetsOfClass "/Game/Menu/MainMenu/WB_MainMenu.WB_MainMenu_C" false))
    (Default|SwitchWidget (Utilities|Array|Get(acopy) _foundwidgets) 3)))

(fn ConstructionScript)